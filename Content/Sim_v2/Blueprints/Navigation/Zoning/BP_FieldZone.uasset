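; BP_FieldZone is a team-assigned zone actor for the sim's navigation zoning, defined by a box and marked with a colored sphere.
; The construction script sizes the box from 2D Dimensions with a fixed height, and tints the sphere with ZoneColor through a dynamic material instance created only when none is valid.
; Preview selection callbacks toggle a Selected flag, and GetTeam exposes the zone's team.
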(event EventBeginPlay)

(event Collision|EventActorBeginOverlap
  (params (OtherActor :type Actor%20Object%20Reference)))

(event EventTick
  (params (DeltaSeconds :type Float%20%28single-precision%29)))

(fn ConstructionScript
  (Utilities|FlowControl|Sequence
    (:then_0
      (Variables|Default|GetDynMI
        (:then)
        (:else
          (bind _returnvalue (Rendering|Material|CreateDynamicMaterialInstance (Variables|Default|GetSphereMat) "None" "None" :!class /Script/Engine.KismetMaterialLibrary))
          (bind _output_get (Variables|Default|SetDynMI _returnvalue))
          (Rendering|Material|SetMaterial (Variables|Default|GetSphere) 0 _output_get))))
    (:then_1
      (Components|Box|SetBoxExtent (Variables|Default|GetBox) (Math|Conversions|ToVector(Vector2D) (Variables|FootballSim|Zoning|GetDimensions) 1.2e+02) false))
    (:then_2
      (Rendering|Material|SetVectorParameterValue (Variables|Default|GetDynMI) "Color" (Variables|FootballSim|Zoning|GetZone%20Color) :!class /Script/Engine.MaterialInstanceDynamic))))

(fn OnSelectedPreview
  (Variables|Default|SetSelected? true))

(fn OnDeselectedPreview
  (Variables|Default|SetSelected? false))

(fn GetTeam
  (return (Variables|FootballSim|Zoning|GetForTeam)))