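; BP_SixYardZone is a navigation zone actor marking a team's six-yard box in the sim.
; The construction script sizes its box component from an Extent variable multiplied by root scale, and selection events show or hide that box.
; Getters expose the zone's team, fixed type and box bounds, though the returned extent is the raw, unscaled value.
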(event EventBeginPlay)

(event Collision|EventActorBeginOverlap
  (params (OtherActor :type Actor%20Object%20Reference)))

(event EventTick
  (params (DeltaSeconds :type Float%20%28single-precision%29)))

(event EventOnSelect
  (Rendering|SetVisibility (Variables|Default|GetBox) true false))

(event EventOnDeSelect
  (Rendering|SetVisibility (Variables|Default|GetBox) false false))

(fn ConstructionScript
  (Components|Box|SetBoxExtent (Variables|Default|GetBox) (* (Variables|FootballSim|Zoning|GetExtent) (Transformation|GetWorldScale (Variables|Default|GetDefaultSceneRoot))) true))

(fn GetZoneBox
  (return (Transformation|GetWorldLocation (Variables|Default|GetBox)) (Variables|FootballSim|Zoning|GetExtent)))

(fn GetZoneTeam
  (return (Variables|FootballSim|Zoning|GetTeam)))

(fn GetZoneType
  (return "NewEnumerator1"))