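; Game mode component that tracks which player currently holds the ball and who held it last.
; Notify functions for receiving, leaving, tackles and shots update CurrentBallHolder and LastBallHolder, then broadcast matching events.
; Tackles cast Defender and Challenger to actors as previous and new holder, printing an error if a cast fails.
; Shots clear the current holder but assign LastBallHolder to itself, so the shooter is not recorded there.
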(event EventBeginPlay)

(event EventTick
  (params (DeltaSeconds :type Float%20%28single-precision%29)))

(fn NotifyPlayerReceiveBall
  (params (Player :type Actor%20Object%20Reference))
  (Variables|Default|SetLastBallHolder (Variables|Default|GetCurrentBallHolder))
  (bind _output_get (Variables|Default|SetCurrentBallHolder Player))
  (Default|CallPlayerReceivedBall _output_get))

(fn NotifyBallLeftPlayer
  (params (LastPlayer :type Actor%20Object%20Reference))
  (Variables|Default|SetLastBallHolder LastPlayer)
  (Variables|Default|SetCurrentBallHolder 0)
  (Default|CallPlayerLeftBall LastPlayer))

(fn NotifyTackleOccurred
  (params (defender :type BI%20Can%20be%20Stolen%20from%20Interface) (challenger :type BI%20Can%20Steal%20Ball%20Interface) (ball :type BI%20Ball%20Interface))
  (Utilities|FlowControl|Sequence
    (:then_0
      (bind _asactor (Utilities|Casting|CastToActor (Utilities|ToObject(Interface) defender))
        (:then
          (Variables|Default|SetLastBallHolder _asactor))
        (:CastFailed
          (Development|PrintString "Ball was stolen from a non-actor (????)" true true "(R=1.000000,G=0.257742,B=0.000000,A=1.000000)"))))
    (:then_1
      (bind _asactor_2 (Utilities|Casting|CastToActor (Utilities|ToObject(Interface) challenger))
        (:then
          (Variables|Default|SetCurrentBallHolder _asactor_2))
        (:CastFailed
          (Development|PrintString "Ball was stolen by a non-actor (????)" true true "(R=1.000000,G=0.257742,B=0.000000,A=1.000000)"))))
    (:then_2
      (Default|CallTackleOccured defender challenger ball))))

(fn NotifyPlayerShotBall
  (params (Shooter :type Controller%20Object%20Reference))
  (Variables|Default|SetLastBallHolder (Variables|Default|GetLastBallHolder))
  (Variables|Default|SetCurrentBallHolder 0)
  (Default|CallPlayerShotBall Shooter))