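; Game mode component that acts as a lookup registry for key actors in the football sim.
; On BeginPlay it caches the single ball and maps each team to its goal, kick locations and kick targets, then signals that references are found.
; Getters read those maps, while team controller and field dimension queries search the world on each call.
; The six-yard zone lookup is an unfinished stub with disconnected logic.
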(event EventBeginPlay
  (Utilities|FlowControl|Sequence
    (:then_0
      (bind _outactors (Actor|GetAllActorswithInterface "/Game/Sim_v2/Blueprints/Core/BI_Ball.BI_Ball_C"))
      (switch int (Utilities|Array|Length _outactors)
        (:Default
          (Development|PrintString "Multiple balls found" true true "(R=1.000000,G=0.000000,B=0.069327,A=1.000000)"))
        (:0
          (Development|PrintString "No ball found" true true "(R=1.000000,G=0.000000,B=0.069327,A=1.000000)"))
        (:1
          (Variables|Debug|SetBall (Utilities|Array|Get(acopy) _outactors)))))
    (:then_1
      (bind _outactors_2 (Actor|GetAllActorswithInterface "/Game/Sim_v2/Blueprints/Goals/BI_Goal.BI_Goal_C"))
      (for _array_element _outactors_2
        (bind _asbi_has_team (Utilities|Casting|CastToBI_HasTeam _array_element))
        (bind _team (Default|GetTeam _asbi_has_team))
        (bind _asactor (Utilities|Casting|CastToActor (Utilities|ToObject(Interface) _asbi_has_team)))
        (Utilities|Map|Add (Variables|Debug|GetFactionToGoal) _team _asactor)))
    (:then_2
      (bind _outactors_3 (Actor|GetAllActorsOfClass "/Game/Sim_v2/Blueprints/Goals/BP_KickLocation.BP_KickLocation_C"))
      (for _array_element_2 _outactors_3
        (bind _team_2 (Default|GetTeam _array_element_2))
        (if (.ReturnValue (Utilities|Map|Find (Variables|Debug|GetFactionToKickLocations) _team_2))
          (Utilities|Array|Add (Utilities|Struct|BreakFKickLocations (.Value (Utilities|Map|Find (Variables|Debug|GetFactionToKickLocations) _team_2))) _array_element_2)
          (Utilities|Map|Add (Variables|Debug|GetFactionToKickLocations) _team_2 (Utilities|Struct|MakeFKickLocations (Utilities|Struct|BreakFKickLocations (.Value (Utilities|Map|Find (Variables|Debug|GetFactionToKickLocations) _team_2)))))
          (else
            (Utilities|Map|Add (Variables|Debug|GetFactionToKickLocations) _team_2 (Utilities|Struct|MakeFKickLocations (Utilities|Array|MakeArray _array_element_2)))))))
    (:then_3
      (bind _outactors_4 (Actor|GetAllActorsOfClass "/Game/Sim_v2/Blueprints/Goals/BP_KickTarget.BP_KickTarget_C"))
      (for _array_element_3 _outactors_4
        (bind _team_3 (Default|GetTeam _array_element_3))
        (if (.ReturnValue (Utilities|Map|Find (Variables|Debug|GetFactionToKickTargets) _team_3))
          (Utilities|Array|Add (Utilities|Struct|BreakFKickTargets (.Value (Utilities|Map|Find (Variables|Debug|GetFactionToKickTargets) _team_3))) _array_element_3)
          (Utilities|Map|Add (Variables|Debug|GetFactionToKickTargets) _team_3 (Utilities|Struct|MakeFKickTargets (Utilities|Struct|BreakFKickTargets (.Value (Utilities|Map|Find (Variables|Debug|GetFactionToKickTargets) _team_3)))))
          (else
            (Utilities|Map|Add (Variables|Debug|GetFactionToKickTargets) _team_3 (Utilities|Struct|MakeFKickTargets (Utilities|Array|MakeArray _array_element_3)))))))
    (:then_4
      (Default|CallReferencesFound))))

(fn GetGoalOfTeam
  (params (Team :type BE_FootballTeam%20Enum :default "NewEnumerator0"))
  (bind _factiontogoal (Variables|Debug|GetFactionToGoal))
  (bind (_value _returnvalue) (Utilities|Map|Find _factiontogoal Team))
  (return _value _returnvalue))

(fn GetKickLocationsOfTeam
  (params (Team :type BE_FootballTeam%20Enum%20%28by%20ref%29 :default "NewEnumerator0"))
  (bind _factiontokicklocations (Variables|Debug|GetFactionToKickLocations))
  (bind (_value _returnvalue) (Utilities|Map|Find _factiontokicklocations Team))
  (return _returnvalue (Utilities|Struct|BreakFKickLocations _value)))

(fn GetKickTargetsOfTeam
  (params (Team :type BE_FootballTeam%20Enum%20%28by%20ref%29 :default "NewEnumerator0"))
  (bind _factiontokicktargets (Variables|Debug|GetFactionToKickTargets))
  (bind (_value _returnvalue) (Utilities|Map|Find _factiontokicktargets Team))
  (return _returnvalue (Utilities|Struct|BreakFKickTargets _value)))

(fn GetControllerOfTeam
  (params (Of%20Team :type BE_FootballTeam%20Enum :default "NewEnumerator0"))
  (bind _outactors (Actor|GetAllActorsOfClass "/Game/Sim_v2/Blueprints/Team/TeamController/AI_TeamController.AI_TeamController_C"))
  (for _array_element _outactors
    (if (Utilities|Enum|Equal(Enum) (Variables|/Game/Sim_v2/Blueprints/Team/TeamController/AI_TeamController.AI_TeamController_C|GetMyTeam _array_element) Of%20Team)
      (return _array_element)))
  (return 0))

(fn GetFieldDimensions
  (bind _returnvalue (Actor|GetActorOfClass "/Game/Sim_v2/Blueprints/Core/A_Field.A_Field_C"))
  (return (Variables|/Game/Sim_v2/Blueprints/Core/A_Field.A_Field_C|GetDimensions _returnvalue)))

(fn GetSixYardZoneOfTeam
  (params (Team :type BE_FootballTeam%20Enum :default "NewEnumerator0")))