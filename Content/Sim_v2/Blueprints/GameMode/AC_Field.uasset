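; AC_Field is a field component that loads the simulation field's configuration from the level's A_FieldSettings actor.
; SettingsFromActor caches that actor and copies its Dimensions, printing a warning if none is found.
; BeginPlay loads the settings and then calls CallFieldInitialized.
; A Preview event also loads them and gathers BI_ListenToFieldPreviewInitialized actors, but its loop over them is empty.
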(event Custom|Preview
  (CallFunction|SettingsfromActor)
  (bind _outactors (Actor|GetAllActorswithInterface "/Game/Sim_v2/Blueprints/Core/BI_ListenToFieldPreviewInitialized.BI_ListenToFieldPreviewInitialized_C"))
  (for _array_element _outactors
    _))

(event EventBeginPlay
  (CallFunction|SettingsfromActor)
  (Default|CallFieldInitialized))

(event EventTick
  (params (DeltaSeconds :type Float%20%28single-precision%29)))

(fn SettingsfromActor
  (bind _returnvalue (Actor|GetActorOfClass "/Game/Sim_v2/Blueprints/Core/A_FieldSettings.A_FieldSettings_C"))
  (bind _output_get (Variables|Debug|SetSettings _returnvalue))
  (Utilities|IsValid _output_get
    (:Is%20Valid
      (bind _output_get_2 (Variables|Debug|SetDimensions (Variables|/Game/Sim_v2/Blueprints/Core/A_FieldSettings.A_FieldSettings_C|GetDimensions (Variables|Debug|GetSettings))))
      (Development|PrintString (Utilities|String|Append "Took dimensions " (Utilities|String|ToString(Vector2d) _output_get_2)) false))
    (:Is%20Not%20Valid
      (Development|PrintString "Cannot preview, no field settings" true true "(R=1.000000,G=0.116351,B=0.000000,A=1.000000)" 2.0 "NO_PREVIEW"))))