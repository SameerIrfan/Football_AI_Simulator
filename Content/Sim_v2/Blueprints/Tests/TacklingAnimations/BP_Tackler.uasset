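; Test actor for a tackling animation that lunges at TackleTarget, treated as the ball, and takes possession of it.
; Tackle yaws toward the target, plays AM_Tackle and drives a timeline lerp in XY to the target's starting position, keeping its own height.
; Once within range, it attaches the target to SCBallAnchor a single time.
; RefreshArrow shows a marker above any valid target, also during construction; GetStealingDistance is a stub.
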(event Custom|Tackle
  (bind _returnvalue (Transformation|GetActorLocation))
  (bind _tackletarget (Variables|FootballSim|Tackle|GetTackleTarget))
  (bind _returnvalue_2 (Transformation|GetActorLocation _tackletarget))
  (Utilities|FlowControl|Sequence
    (:then_0
      (bind _tackletarget_2 (Variables|FootballSim|Tackle|GetTackleTarget)
        (:then
          (Transformation|SetActorRotation (Math|Rotator|MakeRotator 0.0 0.0 (.Yaw (Math|Rotator|BreakRotator (Math|Rotator|MakeRotfromX (- (Transformation|GetActorLocation _tackletarget_2) (Transformation|GetWorldLocation (Variables|Collision|GetCapsuleComponent)))))))))
        (:else)))
    (:then_1
      (Utilities|RefreshArrow))
    (:then_2
      (bind _output_get (Variables|FootballSim|Tackle|SetLocationBeforeTackle (Transformation|GetActorLocation)))
      (Variables|FootballSim|Tackle|SetEndLocation (Transformation|GetActorLocation (Variables|FootballSim|Tackle|GetTackleTarget))))
    (:then_3
      (Components|Animation|PlayAnimation (Variables|Character|GetMesh) "/Game/SoccerAnimations/Montages/AM_Tackle.AM_Tackle" false)
      (bind _tackle_progress (Timeline|TackleTimeline PlayFromStart)
        (:Update
          (Transformation|SetActorLocation (Math|Vector|MakeVector (.X (Math|Vector|BreakVector (Math|Vector|Lerp(Vector) (Variables|FootballSim|Tackle|GetLocationBeforeTackle) (Variables|FootballSim|Tackle|GetEndLocation) _tackle_progress))) (.Y (Math|Vector|BreakVector (Math|Vector|Lerp(Vector) (Variables|FootballSim|Tackle|GetLocationBeforeTackle) (Variables|FootballSim|Tackle|GetEndLocation) _tackle_progress))) (.Z (Math|Vector|BreakVector (Variables|FootballSim|Tackle|GetLocationBeforeTackle)))) false false)
          (Variables|FootballSim|Tackle|SetCurrentDistanceFromBall (Math|Vector|Distance(Vector) _returnvalue_2 (Math|Vector|MakeVector (.x _returnvalue) (.y _returnvalue) (.Z (Math|Vector|BreakVector _returnvalue_2)))))
          (if (< (Variables|FootballSim|Tackle|GetCurrentDistanceFromBall) (Variables|FootballSim|Tackle|GetMaxDistanceToTakeBall))
            (Utilities|FlowControl|DoOnce false
              (:Completed
                (Development|PrintString "Taking ball")
                (Transformation|AttachComponentToComponent (Variables|FootballSim|Tackle|GetTackleTarget) (Variables|Default|GetSC_BallAnchor) "None" "SnapToTarget" "KeepRelative" "KeepRelative" true)))))))))

(event EventBeginPlay)

(event Collision|EventActorBeginOverlap
  (params (OtherActor :type Actor%20Object%20Reference)))

(event EventTick
  (params (DeltaSeconds :type Float%20%28single-precision%29)))

(fn ConstructionScript
  (Utilities|FlowControl|Sequence
    (:then_1
      (Utilities|RefreshArrow))))

(fn GetStealingDistance
  (return 0.0))