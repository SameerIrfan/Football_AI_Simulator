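; AI controller for a simulated football player that runs the BT_Scorer behavior tree, seeding its blackboard with ball and team.
; It relays take, steal and shoot actions to the pawn, reporting possession changes, tackles and shots to the GameMode's BallOwnerTracker component.
; It exposes player and zone queries, plus a distance-based ball pursuit cost that becomes prohibitive during cooldowns.
; Several getters are zero-returning stubs, and the kick-location blackboard setup is disconnected.
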(event Custom|On%20Character%20Stealing%20Complete
  (params (defender :type BI%20Can%20be%20Stolen%20from%20Interface) (ball :type BI%20Ball%20Interface))
  (Default|BeStolenfrom defender self ball)
  (Default|NotifyTackleOccurred (Variables|Default|GetBallOwnerTrackerRef) defender self ball))

(event EventBeginPlay
  (bind _returnvalue (Pawn|GetControlledPawn))
  (bind _returnvalue_2 (Game|GetGameMode))
  (bind _returnvalue_3 (Game|GetGameMode))
  (bind _returnvalue_4 (Actor|GetComponentbyClass _returnvalue_2 "/Game/Sim_v2/Blueprints/GameMode/AC_BallOwnerTracker.AC_BallOwnerTracker_C"))
  (bind _returnvalue_5 (Actor|GetComponentbyClass _returnvalue_3 "/Game/Sim_v2/Blueprints/GameMode/AC_GameReferences.AC_GameReferences_C"))
  (Utilities|FlowControl|Sequence
    (:then_0
      (bind _asbp_football_player_base (Utilities|Casting|CastToBP_FootballPlayer_Base _returnvalue)
        (:then
          (bind _output_get (Variables|Default|SetFootballPlayerRef _asbp_football_player_base))
          (bind _asbi_has_team (Utilities|Casting|CastToBI_HasTeam _output_get)
            (:then
              (bind _team (Default|GetTeam _asbi_has_team))
              (Variables|Sim|Debug|SetTeam _team)
              (EventDispatchers|BindEventtoStealingComplete (Variables|Default|GetFootballPlayerRef) (delegate Custom|On%20Character%20Stealing%20Complete)))
            (:CastFailed
              (Development|PrintString (Utilities|String|Append "AI_FootballController assigned to Pawn " (Utilities|GetDisplayName _returnvalue) " that does not implement BI_Team")))))
        (:CastFailed
          (Development|PrintString "AI Controller not attached to a BP_FootballPlayer_Base" true true "(R=1.000000,G=0.102567,B=0.000000,A=1.000000)" 99.0))))
    (:then_1
      (Utilities|IsValid _returnvalue_5
        (:Is%20Valid
          (Variables|Default|SetGameReferencesRef _returnvalue_5))
        (:Is%20Not%20Valid
          (Development|PrintString "No GameReferences found in GameMode" true true "(R=1.000000,G=0.014042,B=0.000000,A=1.000000)"))))
    (:then_2
      (Utilities|FlowControl|DelayUntilNextTick)
      (AI|RunBehaviorTree "/Game/Sim_v2/Blueprints/AI/Behavior/BT_Scorer.BT_Scorer")
      (Utilities|FlowControl|Sequence
        (:then_0
          (AI|Components|Blackboard|SetValueasObject (AI|GetBlackboard 0) (Variables|BehaviorTree|Keys|GetInKey_Ball) (Variables|/Game/Sim_v2/Blueprints/GameMode/AC_GameReferences.AC_GameReferences_C|GetBall (Variables|Default|GetGameReferencesRef)))
          (AI|Components|Blackboard|SetValueasEnum (AI|GetBlackboard 0) (Variables|BehaviorTree|Keys|GetInKey_Team) (Variables|Sim|Debug|GetTeam)))
        (:then_1
          (Utilities|IsValid _returnvalue_4
            (:Is%20Valid
              (Variables|Default|SetBallOwnerTrackerRef _returnvalue_4))
            (:Is%20Not%20Valid
              (Development|PrintString "No PlayerHasBall Component in Game Mode" true true "(R=1.000000,G=0.024798,B=0.000000,A=1.000000)"))))))
    (:then_3)))

(event EventTick
  (params (DeltaSeconds :type Float%20%28single-precision%29)))

(event EventStartStealfrom
  (params (defender :type BI%20Can%20be%20Stolen%20from%20Interface) (ball :type BI%20Ball%20Interface))
  (Default|StartStealfrom (Variables|Default|GetFootballPlayerRef) defender ball))

(event EventBeStolenfrom
  (params (challenger :type BI%20Can%20Steal%20Ball%20Interface) (ball :type BI%20Ball%20Interface))
  (bind _asbi_can_be_stolen_from (Utilities|Casting|CastToBI_CanBeStolenFrom (Pawn|GetControlledPawn)))
  (Default|BeStolenfrom _asbi_can_be_stolen_from challenger ball))

(event EventLeaveBall
  (Default|NotifyBallLeftPlayer (Variables|Default|GetBallOwnerTrackerRef) self))

(event EventTakeBall
  (params (Ball :type BI%20Ball%20Interface))
  (Default|TakeBall (Variables|Default|GetFootballPlayerRef) Ball)
  (Default|NotifyPlayerReceiveBall (Variables|Default|GetBallOwnerTrackerRef) self))

(fn ConstructionScript)

(fn GetBallPursuitCost
  (Utilities|FlowControl|Sequence
    (:then_0
      (if (.Value (Utilities|Map|Find (Variables|Sim|Debug|GetCooldowns) "NewEnumerator0"))
        (return 999999.0)))
    (:then_1
      (if (.Value (Utilities|Map|Find (Variables|Sim|Debug|GetCooldowns) "NewEnumerator1"))
        (return 999999.0)))
    (:then_2
      (LocalVariables|SettempCost (+ (Math|Vector|Distance(Vector) (Transformation|GetActorLocation (Pawn|GetControlledPawn)) (Transformation|GetActorLocation (Variables|/Game/Sim_v2/Blueprints/GameMode/AC_GameReferences.AC_GameReferences_C|GetBall (Variables|Default|GetGameReferencesRef)))) (LocalVariables|GettempCost))))
    (:then_3
      (return (LocalVariables|GettempCost)))))

(fn SetCooldown
  (params (CooldownName :type FootballCooldown%20Enum%20%28by%20ref%29 :default "NewEnumerator0") (CooldownNewValue :type Boolean))
  (Utilities|Map|Add (Variables|Sim|Debug|GetCooldowns) CooldownName CooldownNewValue))

(fn GetSixYardZone
  (bind _zone (Default|GetSixYardZoneOfTeam (Variables|Default|GetGameReferencesRef) (Variables|Sim|Debug|GetTeam)))
  (return _zone))

(fn GetSixYardBox
  (bind _zone (Default|GetSixYardZoneOfTeam (Variables|Default|GetGameReferencesRef) (Variables|Sim|Debug|GetTeam)))
  (bind (_origin _extent) (Default|GetZoneBox _zone))
  (return _origin _extent))

(fn GetBallOwningDistanceOld
  (return 0.0))

(fn GetBallOwningDistance
  (return 0.0))

(fn GetCost
  (return 0.0))

(fn GetSixYardBoxExtents
  (return "0, 0, 0"))

(fn GetSixYardBoxOrigin
  (bind _origin (CallFunction|GetSixYardBox))
  (return _origin))

(fn GetStealingDistance
  (return (Variables|/Game/Sim_v2/Blueprints/Players/BP_FootballPlayer_Base.BP_FootballPlayer_Base_C|GetStealingDistance (Variables|Default|GetFootballPlayerRef))))

(fn GetTeam
  (return (Variables|/Game/Sim_v2/Blueprints/Players/BP_FootballPlayer_Base.BP_FootballPlayer_Base_C|GetTeam (Variables|Default|GetFootballPlayerRef))))

(fn GetZoneCenter
  (bind _center (Default|GetZoneCenter (Variables|Default|GetFootballPlayerRef)))
  (return _center))

(fn GetZoneRadius
  (bind _dimensions (Default|GetZoneRadius (Variables|Default|GetFootballPlayerRef)))
  (return _dimensions))

(fn StartShootTowards
  (params (Target%20Location :type Vector :default "0, 0, 0"))
  (Default|StartShootTowards (Variables|Default|GetFootballPlayerRef) Target%20Location)
  (Default|NotifyPlayerShotBall (Variables|Default|GetBallOwnerTrackerRef) self))