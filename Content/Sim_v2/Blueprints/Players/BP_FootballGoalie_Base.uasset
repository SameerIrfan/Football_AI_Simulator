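; Base football goalie character that takes, shoots and steals the ball, with a team and a wandering zone.
; Taking the ball snaps it to an anchor and changes walk speed; shots play a montage, with FinishShot detaching and launching the ball.
; Steals use a timeline-driven tackle slide that teleports toward the ball and takes it within range.
; Construction sets up the zone sphere; several ball, speed and distance getters return placeholder values.
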(event EventTakeBall
  (params (Ball :type BI%20Ball%20Interface))
  (Variables|FootballSim|Stealing|Debug|SetHasBall true)
  (bind _asactor (Utilities|Casting|CastToActor (Utilities|ToObject(Interface) Ball))
    (:then
      (Variables|FootballSim|SetAttached%20Ball%20Actor _asactor)
      (Default|OnTake Ball self)
      (Transformation|AttachComponentToComponent _asactor (Variables|Default|GetSC_BallAnchor) "None" "SnapToTarget" "KeepWorld" "KeepWorld" true)
      (Variables|/Script/Engine.CharacterMovementComponent|SetMaxWalkSpeed (Variables|Character|GetCharacterMovement) (Variables|FootballSim|CharacterSettings|GetMax%20Movement%20Speed%20With%20Ball))
      (Transformation|SetActorLocation _asactor (Transformation|GetWorldLocation (Variables|Default|GetSC_BallAnchor)) false true))
    (:CastFailed
      (Development|PrintString "Ball is not an actor, cannot attach"))))

(event EventStartShootTowards
  (params (Target%20Location :type Vector :default "0, 0, 0"))
  (Variables|FootballSim|SetShotTarget Target%20Location)
  (Animation|Montage|PlayMontage (Variables|Character|GetMesh) (Variables|FootballSim|CharacterSettings|GetShootMontage) 1.0 0.0 "ShootNormal"))

(event EventLeaveBall
  (Variables|FootballSim|Stealing|Debug|SetHasBall false))

(event EventStartStealfrom
  (params (defender :type BI%20Can%20be%20Stolen%20from%20Interface) (ball :type BI%20Ball%20Interface))
  (bind _returnvalue (Transformation|GetActorLocation))
  (bind (_x _y) (Math|Vector|BreakVector _returnvalue))
  (if (not (Variables|FootballSim|Stealing|Debug|GetIsTackling))
    (bind _asactor (Utilities|Casting|CastToActor (Utilities|ToObject(Interface) ball)))
    (Variables|FootballSim|Stealing|Debug|SetBallLocationForTackle (Transformation|GetActorLocation _asactor))
    (Variables|FootballSim|Stealing|Debug|SetSelfLocationBeforeTackle (Transformation|GetActorLocation))
    (Variables|FootballSim|Stealing|Debug|SetIsTackling true)
    (Animation|PlayAnimMontage (Variables|FootballSim|Stealing|GetTackleMontage) 1.0 "TackleSlide")
    (bind _tackling_progress (Timeline|Tackling%20Timeline PlayFromStart)
      (:Update
        (Transformation|SetActorLocation (Math|Vector|MakeVector (.x (Math|Vector|Lerp(Vector) (Variables|FootballSim|Stealing|Debug|GetSelfLocationBeforeTackle) (Math|Vector|SelectVector (Variables|FootballSim|Stealing|Debug|GetBallLocationForTackle) (Transformation|GetActorLocation _asactor) (Variables|FootballSim|Stealing|Debug|GetHasBall)) _tackling_progress)) (.y (Math|Vector|Lerp(Vector) (Variables|FootballSim|Stealing|Debug|GetSelfLocationBeforeTackle) (Math|Vector|SelectVector (Variables|FootballSim|Stealing|Debug|GetBallLocationForTackle) (Transformation|GetActorLocation _asactor) (Variables|FootballSim|Stealing|Debug|GetHasBall)) _tackling_progress)) (.Z (Math|Vector|BreakVector (Variables|FootballSim|Stealing|Debug|GetSelfLocationBeforeTackle)))) false true)
        (if (< (Math|Vector|Distance2D(Vector) (Math|Vector2D|MakeVector2D (.x (Transformation|GetActorLocation _asactor)) (.y (Transformation|GetActorLocation _asactor))) (Math|Vector2D|MakeVector2D _x _y)) (Variables|FootballSim|CharacterSettings|GetTackleBallTakingDistance))
          (Utilities|FlowControl|DoOnce false :!label _label
            (:Completed
              (CallFunction|TakeBall ball)
              (Variables|FootballSim|Stealing|Debug|SetHasBall true)
              (Default|CallStealingComplete defender ball)
              (Variables|/Script/Engine.CharacterMovementComponent|SetMaxWalkSpeed (Variables|Character|GetCharacterMovement) (Variables|FootballSim|CharacterSettings|GetMax%20Movement%20Speed%20With%20Ball))))))
      (:Finished
        (Utilities|FlowControl|Sequence
          (:then_0
            (goto _label Reset))
          (:then_1
            (Variables|FootballSim|Stealing|Debug|SetIsTackling false)
            (Animation|StopAnimMontage (Variables|FootballSim|Stealing|GetTackleMontage))))))))

(event EventBeStolenfrom
  (params (challenger :type BI%20Can%20Steal%20Ball%20Interface) (ball :type BI%20Ball%20Interface))
  (Variables|/Script/Engine.CharacterMovementComponent|SetMaxWalkSpeed (Variables|Character|GetCharacterMovement) (Variables|FootballSim|CharacterSettings|GetDefault%20Max%20Movement%20Speed))
  (Animation|PlayAnimMontage (Variables|FootballSim|Stealing|GetBeTackledMontage) 1.0 "TackleL")
  (Default|CallBallWasJustStolenfromMe challenger))

(event EventFinishShot
  (bind _attached_ball_actor (Variables|FootballSim|GetAttached%20Ball%20Actor))
  (Transformation|DetachFromActor _attached_ball_actor "KeepWorld" "KeepWorld" "KeepWorld")
  (Class|BIBall|OnLeave(Message) _attached_ball_actor)
  (Class|BIBall|Shoot(Message) _attached_ball_actor (Variables|FootballSim|GetShotTarget))
  (Variables|/Script/Engine.CharacterMovementComponent|SetMaxWalkSpeed (Variables|Character|GetCharacterMovement) (Variables|FootballSim|CharacterSettings|GetDefault%20Max%20Movement%20Speed)))

(fn ConstructionScript
  (bind _sphere (Variables|Default|GetSphere))
  (Components|Sphere|SetSphereRadius (Variables|Default|GetSphere) (Variables|FootballSim|CharacterSettings|GetWanderingRadius) true)
  (if (Variables|FootballSim|CharacterSettings|GetWanderingOriginFromStartLocation)
    (Transformation|SetRelativeLocation _sphere "0, 0, 0" false false)
    (Variables|FootballSim|CharacterSettings|SetWanderingOrigin (Transformation|GetWorldLocation _sphere))
    (else
      (Transformation|SetWorldLocation (Variables|Default|GetSphere) (Variables|FootballSim|CharacterSettings|GetWanderingOrigin) false false))))

(fn GetBallOwningDistance
  (return 0.0))

(fn GetCurrentSpeed
  (return 0.0))

(fn GetHasBall
  (return false))

(fn GetMaxSpeed
  (return (Class|MovementComponent|GetMaxSpeed (Variables|Character|GetCharacterMovement))))

(fn GetStealingDistance
  (return 0.0))

(fn GetTeam
  (return (Variables|FootballSim|Team|GetTeam)))

(fn GetZoneCenter
  (return (Variables|FootballSim|CharacterSettings|GetWanderingOrigin)))

(fn GetZoneRadius
  (return (Variables|FootballSim|CharacterSettings|GetWanderingRadius)))