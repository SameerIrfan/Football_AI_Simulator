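; Physics ball actor that can be taken, released and shot toward a target point.
; OnTake stops physics simulation and constrains the mesh to the YZ plane, while OnLeave clears the constraint and re-enables simulation.
; Shoot turns collision back on and applies an impulse toward the target that scales with distance, without itself enabling physics.
; Delayed upward force and debug box nodes are left unconnected.
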(event EventBeginPlay)

(event Collision|EventActorBeginOverlap
  (params (OtherActor :type Actor%20Object%20Reference)))

(event EventTick
  (params (DeltaSeconds :type Float%20%28single-precision%29)))

(event EventShoot
  (params (Target :type Vector :default "0, 0, 0"))
  (bind _returnvalue (Transformation|GetActorLocation))
  (bind _returnvalue_2 (- Target _returnvalue))
  (Utilities|FlowControl|Sequence
    (:then_1
      (Collision|SetCollisionEnabled (Variables|Default|GetBallMesh) "QueryAndPhysics")
      (Physics|AddImpulse (Variables|Default|GetBallMesh) (* (Math|Vector|Normalize _returnvalue_2) (Math|Conversions|ToVector(Float) 5.0) (Math|Vector|VectorLength _returnvalue_2)) "None" false))))

(event EventOnLeave
  (Class|PrimitiveComponent|SetConstraintMode (Variables|Default|GetBallMesh) "None")
  (Physics|SetSimulatePhysics (Variables|Default|GetBallMesh) true))

(fn ConstructionScript)

(fn OnTake
  (params (Taker :type Object%20Object%20Reference))
  (bind _ballmesh (Variables|Default|GetBallMesh))
  (Class|PrimitiveComponent|SetConstraintMode _ballmesh "YZPlane")
  (Physics|SetSimulatePhysics _ballmesh false))