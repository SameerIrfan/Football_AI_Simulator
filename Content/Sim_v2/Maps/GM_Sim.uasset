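; GM_Sim is the game mode for the Sim_v2 simulation, driving a ball-and-goal round through its start, active and goal-scored phases.
; BeginPlay steps ACGameStateController through two states with a short delay between, then binds to the ball-entered event of every BP_Goal.
; A goal sets a third state and, after a pause, reloads the current level.
; The construction script calls Preview on the ACField component.
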(event Custom|On%20Ball%20Entered%20Goal
  (params (Goal :type BP%20Goal%20Object%20Reference))
  (Default|SetGameState (Variables|Default|GetAC_GameStateController) "NewEnumerator2")
  (Utilities|FlowControl|Delay 2.0)
  (bind _returnvalue (Game|GetCurrentLevelName true))
  (Game|OpenLevel(byName) (Utilities|String|StringToName _returnvalue)))

(event EventBeginPlay
  (Default|SetGameState (Variables|Default|GetAC_GameStateController) "NewEnumerator0")
  (Utilities|FlowControl|Delay 2.0)
  (Default|SetGameState (Variables|Default|GetAC_GameStateController) "NewEnumerator1")
  (bind _outactors (Actor|GetAllActorsOfClass "/Game/Sim_v2/Blueprints/Goals/BP_Goal.BP_Goal_C"))
  (for _array_element _outactors
    (EventDispatchers|BindEventtoBallEntered _array_element (delegate Custom|On%20Ball%20Entered%20Goal))))

(event EventTick
  (params (DeltaSeconds :type Float%20%28single-precision%29)))

(fn ConstructionScript
  (Default|Preview (Variables|Default|GetAC_Field)))