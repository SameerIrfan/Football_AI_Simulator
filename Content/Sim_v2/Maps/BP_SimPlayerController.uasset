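; Player controller for the Sim_v2 game that prints the name of each pawn it possesses and provides a lookup for the player's six-yard box.
; GetPlayerSixYardBox returns the reference held in ACSixYardZone when valid.
; Otherwise it prints a warning, scans all TriggerVolumes for the first carrying an AC_SixYardZone component, then caches and returns that volume.
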(event EventBeginPlay)

(event EventTick
  (params (DeltaSeconds :type Float%20%28single-precision%29)))

(event EventPossess
  (params (PossessedPawn :type Pawn%20Object%20Reference))
  (|CallParentFunction PossessedPawn)
  (Development|PrintText (Utilities|Text|FormatText "Possessed {0}" (Utilities|GetDisplayName PossessedPawn))))

(fn ConstructionScript)

(fn GetPlayerSixYardBox
  (bind _ac_sixyardzone (Variables|Default|GetAC_SixYardZone))
  (bind _playersixyardbox (Variables|/Game/Sim_v2/Blueprints/Goals/AC_SixYardZone.AC_SixYardZone_C|GetPlayerSixYardBox _ac_sixyardzone)
    (:then
      (return _playersixyardbox))
    (:else
      (Development|PrintString "Player Six yar Box is not Valid Setting")
      (bind _outactors (Actor|GetAllActorsOfClass "/Script/Engine.TriggerVolume"))
      (bind _array_element (Utilities|Array|ForEachLoopwithBreak _outactors)
        (:LoopBody
          (Utilities|IsValid (Actor|GetComponentbyClass _array_element "/Game/Sim_v2/Blueprints/Goals/AC_SixYardZone.AC_SixYardZone_C")
            (:Is%20Valid
              (Variables|/Game/Sim_v2/Blueprints/Goals/AC_SixYardZone.AC_SixYardZone_C|SetPlayerSixYardBox _ac_sixyardzone _array_element)
              (return _array_element))))))))