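; BP_SimPawn is a camera pawn that follows and frames a target actor, ToTrack.
; Each Tick and the construction script call AdjustCamera, which, when ToTrack is valid, moves the pawn onto the target.
; It then sets CorrectCam at OffsetFromTarget relative to its parent and rotates it to look at the target.
; Becoming the view target only prints a debug string.
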(event EventBeginPlay)

(event Collision|EventActorBeginOverlap
  (params (OtherActor :type Actor%20Object%20Reference)))

(event EventTick
  (params (DeltaSeconds :type Float%20%28single-precision%29))
  (CallFunction|AdjustCamera))

(event EventOnBecomeViewTarget
  (params (PC :type Player%20Controller%20Object%20Reference))
  (Development|PrintString "Im supposed to be the view target"))

(fn ConstructionScript
  (CallFunction|AdjustCamera))

(fn AdjustCamera
  (bind _totrack (Variables|FootballSim|GetToTrack)
    (:then
      (Transformation|SetActorLocation (Transformation|GetActorLocation _totrack) false false)
      (Transformation|SetRelativeLocation (Variables|Default|GetCorrectCam) (Variables|FootballSim|GetOffsetFromTarget) false false)
      (Transformation|SetWorldRotation (Variables|Default|GetCorrectCam) (Math|Rotator|FindLookatRotation (Transformation|GetWorldLocation (Variables|Default|GetCorrectCam)) (Transformation|GetActorLocation _totrack)) true false))
    (:else)))