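; BP_SimPawnSettings is a camera-rig actor for the sim maps, apparently used to set up and preview a view of a TrackTarget.
; Its construction script teleports the actor onto a valid target, applies Offset to the spring arm, and derives the arm's rotation from the PreviewCam look-at plus Rotation.
; All work happens at construction; the event graph holds only disabled stubs.
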(event EventBeginPlay)

(event Collision|EventActorBeginOverlap
  (params (OtherActor :type Actor%20Object%20Reference)))

(event EventTick
  (params (DeltaSeconds :type Float%20%28single-precision%29)))

(fn ConstructionScript
  (bind _tracktarget (Variables|FootballSim|GetTrackTarget)
    (:then
      (Transformation|SetActorLocation (Transformation|GetActorLocation _tracktarget) false true)
      (Variables|/Script/Engine.SpringArmComponent|SetTargetOffset (Variables|Default|GetSpringArm) (Variables|FootballSim|GetOffset))
      (Transformation|SetRelativeRotation (Variables|Default|GetSpringArm) (Math|Conversions|RotationFromXVector (+ (Math|Rotator|FindLookatRotation (Transformation|GetWorldLocation (Variables|Default|GetPreviewCam)) (Transformation|GetActorLocation _tracktarget)) (Variables|FootballSim|GetRotation))) false false))
    (:else)))